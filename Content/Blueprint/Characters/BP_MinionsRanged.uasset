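; BP_MinionsRanged is an AI minion that wanders, chases the Khaimera player character and dies when its health runs out.
; A self-repeating AIMoveTo roams nearby random navigable points, while PawnSensing sightings start a move toward the player.
; Reaching the player sets IsPunching, cleared after a delay if not touching.
; Despite the name, damage comes from Gauche component overlaps, and incoming damage lowers VieAi until the actor is destroyed.
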(event `self.ReceiveBeginPlay`
  (`self.IA MooveRandomPoint`))

(event `IA MoveToPlayer`
  (params (Pawn :type "Pawn Object Reference"))
  (`|AIMoveTo` self (0.0 0.0 0.0) Pawn 230.0
    (:`OnSuccess`
      (set `self.isPunching` true)
      (if (not (`self.isTouching`))
        (`KismetSystemLibrary.Delay` 6.0)
        (set `self.isPunching` false)
        (set `self.IASeePlayer` false)))))

(event `IA MooveRandomPoint`
  ;[1 1 1] Deplacement
  (if (not (`self.IASeePlayer`))
    (`|AIMoveTo` self (`NavigationSystemV1.K2_GetRandomLocationInNavigableRadius` (`self.K2_GetActorLocation`) 300.0 null null) null
      (:`OnSuccess`
        (`self.IA MooveRandomPoint`)))))

(event `self.PawnSensing.OnSeePawn`
  (params (Pawn :type "Pawn Object Reference"))
  ;[1 1 1] Deplacement
  (bind _askhaimera_player_character (cast `/Game/Blueprint/Characters/KhaimeraPlayerCharacter` Pawn))
  (set `self.IASeePlayer` false)
  (`self.IA MoveToPlayer` _askhaimera_player_character))

(event `self.Gauche.OnComponentBeginOverlap`
  (params (OverlappedComponent :type "PrimitiveComponent Object Reference") (OtherActor :type "Actor Object Reference") (OtherComp :type "PrimitiveComponent Object Reference") (OtherBodyIndex :type Integer) (bFromSweep :type Boolean) (SweepResult :type "HitResult Structure (by ref)"))
  (bind _returnvalue (`GameplayStatics.GetPlayerCharacter` 0))
  ;[1 1 1] Apply Damage
  (if (== OtherActor _returnvalue)
    (if (`PrimitiveComponent.IsOverlappingActor` (`self.Gauche`) (`GameplayStatics.GetPlayerCharacter` 0))
      (`GameplayStatics.ApplyDamage` _returnvalue 20.0 null null "/Script/Engine.DamageType"))))

(event `self.ReceiveAnyDamage`
  (params (Damage :type "Float (single-precision)") (DamageType :type "DamageType Object Reference") (InstigatedBy :type "Controller Object Reference") (DamageCauser :type "Actor Object Reference"))
  ;[1 1 1] Gestion Degats
  (bind _output_get (set `self.VieAi` (- (`self.VieAi`) (`KismetMathLibrary.FTrunc` Damage))))
  (if (<= _output_get 0)
    (`KismetSystemLibrary.PrintString` "t dead")
    (`self.K2_DestroyActor`)))

(fn `GestionVieAi`
  (params (PointsVieAi :type Integer))
  (set `self.VieAi` (+ (`self.VieAi`) PointsVieAi)))

(fn `UserConstructionScript`)
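; Weather controller for the meadow map that randomly switches between clear skies and rainstorms that bring ranged minion enemies.
; After a startup delay it begins a storm if the sky reference is valid, while a looping timer randomly chooses storm or clearing.
; Storms use a timeline to darken sky material and light, activate rain particles and audio, and spawn minions near the player.
; Clearing deactivates the rain and reverses the timeline.
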(event `self.ReceiveBeginPlay`
  (bind _returnvalue (`KismetMathLibrary.RandomFloatInRange` 200.0 400.0))
  (bind _rain (`self.rain`))
  (bind (_returnvalue_x _returnvalue_y _returnvalue_z) (`KismetMathLibrary.BreakVector` (`self.K2_GetActorLocation` (`GameplayStatics.GetPlayerCharacter` 0))))
  (bind _sky_material (`/Engine/EngineSky/BP_Sky_Sphere.Sky material` (`self.SkyRef`)))
  (bind _particlesystemcomponent (`Emitter.ParticleSystemComponent` (`self.RainRef`)))
  (`KismetSystemLibrary.Delay` 120.0)
  (`KismetSystemLibrary.K2_SetTimerDelegate` (delegate `Weather`) 157.0 true)
  (if (`KismetSystemLibrary.IsValid` (`self.SkyRef`))
    (`/Engine/EditorBlueprintResources/StandardMacros.FlipFlop`
      (:`A`
        (`|ExecutionSequence` :!label _label
          (:`then_0`
            (bind (_direction _newtrack_1) (`Timeline|Timeline_0` :!label _label_2)
              (:`Update`
                (`MaterialInstanceDynamic.SetVectorParameterValue` _sky_material "Zenith Color" (`KismetMathLibrary.LinearColorLerp` (struct :`G` 0.136337 :`B` 0.229167 :`A` 1.0) (struct :`R` 0.125 :`G` 0.125 :`B` 0.125 :`A` 1.0) _newtrack_1))
                (`MaterialInstanceDynamic.SetVectorParameterValue` _sky_material "Horizon Color" (`KismetMathLibrary.LinearColorLerp` (struct :`R` 0.855778 :`G` 0.91902 :`B` 2.0 :`A` 1.0) (struct :`R` 0.020833 :`G` 0.020833 :`B` 0.020833 :`A` 1.0) _newtrack_1))
                (`MaterialInstanceDynamic.SetVectorParameterValue` _sky_material "Cloud Color" (`KismetMathLibrary.LinearColorLerp` (struct :`R` 1.0 :`G` 1.0 :`B` 1.0 :`A` 1.0) (struct :`R` 0.020833 :`G` 0.020833 :`B` 0.020833 :`A` 1.0) _newtrack_1))
                (`MaterialInstanceDynamic.SetScalarParameterValue` _sky_material "Cloud Opacity" (`KismetMathLibrary.Lerp` 1.2 4.0 _newtrack_1))
                (`LightComponent.SetLightColor` (`Light.LightComponent` (`self.LightRef`)) (`KismetMathLibrary.LinearColorLerp` (struct :`R` 1.0 :`G` 1.0 :`B` 1.0 :`A` 1.0) (struct :`R` 0.020833 :`G` 0.020833 :`B` 0.020833 :`A` 1.0) _newtrack_1) true))))
          (:`then_1`
            (`KismetSystemLibrary.Delay` 1.0)
            (`ActorComponent.Activate` _particlesystemcomponent false))
          (:`then_2`
            (`KismetSystemLibrary.Delay` 3.0)
            (`AudioComponent.Play` _rain 0.0)
            (`KismetSystemLibrary.Delay` 157.0)
            (`AudioComponent.Stop` _rain))
          (:`then_3`
            (for _ (range (+ (`KismetMathLibrary.RandomIntegerInRange` 2 6) 1))
              (`|SpawnActorFromClass` "/Game/Blueprint/Characters/BP_MinionsRanged.BP_MinionsRanged_C" (`KismetMathLibrary.MakeTransform` (`KismetMathLibrary.MakeVector` (+ _returnvalue_x _returnvalue) (+ _returnvalue_y _returnvalue) _returnvalue_z)) "Undefined" "OverrideRootScale" null null)))))
      (:`B`
        (`ActorComponent.Deactivate` _particlesystemcomponent :!label _label_3)
        (`KismetSystemLibrary.Delay` 1.0)
        (goto _label_2 :!via `Reverse`)))))

(event `Weather`
  (if (== (`KismetMathLibrary.RandomIntegerInRange` 0 2) 1)
    (goto _label)
    (else
      (goto _label_3))))

(fn `UserConstructionScript`)